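; Game mode for Carom that picks a player start according to the player's team.
; BeginPlay fills the Team A and Team B spawn arrays through GetTeamSpawns, which finds PlayerStarts by gameplay tag query and returns inside its loop after the first match.
; ChoosePlayerStart reads TeamId from the CaromPlayerController, giving team zero the first Team A spawn and any other team the first Team B spawn.
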(event EventBeginPlay
  (bind _starts1 (CallFunction|GetTeamSpawns))
  (Variables|Default|SetTeamASpawns _starts1)
  (bind _starts1_2 (CallFunction|GetTeamSpawns))
  (Variables|Default|SetTeamBSpawns _starts1_2))

(event EventTick
  (params (DeltaSeconds :type Float%20%28single-precision%29)))

(fn ConstructionScript)

(fn ChoosePlayerStart
  (params (Player :type Controller%20Object%20Reference))
  (bind _ascarom_player_controller (Utilities|Casting|CastToCaromPlayerController Player))
  (Math|Integer|CompareInt (Variables|/Game/Blueprints/CaromPlayerController.CaromPlayerController_C|GetTeamId _ascarom_player_controller) 0
    (:>
      _)
    (:==
      (return (Utilities|Array|Get(acopy) (Variables|Default|GetTeamASpawns))))
    (:<
      _))
  (return (Utilities|Array|Get(acopy) (Variables|Default|GetTeamBSpawns))))

(fn GetTeamSpawns
  (params (GameplayTagQuery :type Gameplay%20Tag%20Query%20Structure%20%28by%20ref%29))
  (bind _starts (LocalVariables|Getstarts))
  (bind _outactors (Class|BlueprintGameplayTagLibrary|GetAllActorsOfClassMatchingTagQuery "/Script/Engine.PlayerStart" GameplayTagQuery))
  (for _array_element _outactors
    (bind _asplayer_start (Utilities|Casting|CastToPlayerStart _array_element))
    (Utilities|Array|Add _starts _asplayer_start)
    (return _starts)))